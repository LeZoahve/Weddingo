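; Player pawn that appears as either a red panda or an otter, depending on the controlling player's index.
; On possession it looks up that index through BP_GameState, then sets the matching skeletal mesh and animation Blueprint.
; It also copies its scale from the BP_PlayerStart with the same index and the first Scene enum value.
; PlayAnim forwards animation requests to the mesh's anim instance as a message.
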(event `self.ReceivePossessed`
  (params (NewController :type "Controller Object Reference"))
  (bind _playerindex (`self.GetPlayerIndex`))
  (`SkeletalMeshComponent.SetSkeletalMeshAsset` (`self.SkeletalMesh`) (select `int` _playerindex :`0` "/Game/Meshes/Core/Red_Panda.Red_Panda" :`1` "/Game/Meshes/Core/Otter.Otter" :!type "SkeletalMesh Object Reference"))
  (`SkeletalMeshComponent.SetAnimInstanceClass` (`self.SkeletalMesh`) (select `int` _playerindex :`0` "/Game/Blueprints/Anim/ABP_Panda.ABP_Panda_C" :`1` "/Game/Blueprints/Anim/ABP_Otter.ABP_Otter_C" :!type "Object Class Reference"))
  (bind _return_value_scale (`self.GetInitialScale`))
  (`self.SetActorScale3D` _return_value_scale))

(fn `GetInitialScale`
  (returns (`Return Value Scale` :type "Vector Structure"))
  (bind _playerindex (`self.GetPlayerIndex`))
  (bind _outactors (`GameplayStatics.GetAllActorsOfClass` "/Game/Blueprints/BP_PlayerStart.BP_PlayerStart_C"))
  (for _array_element _outactors
    (if (and (== (`/Game/Blueprints/BP_PlayerStart.playerIndex` _array_element) _playerindex) (`|EnumEquality` (`/Game/Blueprints/BP_PlayerStart.Scene` _array_element) "NewEnumerator0"))
      (bind (_returnvalue_location _returnvalue_rotation _returnvalue_scale) (`KismetMathLibrary.BreakTransform` (`self.GetTransform` _array_element)))
      (return _returnvalue_scale))))

(fn `GetPlayerIndex`
  (returns (PlayerIndex :type Integer))
  (bind _asbp_game_state (cast `/Game/Blueprints/BP_GameState` (`GameplayStatics.GetGameState`)))
  (bind _asbp_player_controller (cast `/Game/Blueprints/BP_PlayerController` (`self.GetController` self))
    (:`then`
      (bind _playerindex (`/Game/Blueprints/BP_GameState.GetPlayerIndex` _asbp_game_state _asbp_player_controller)))
    (:`CastFailed`
      _))
  (return _playerindex))

(fn `PlayAnim`
  (params (Animation :type "/Game/Enum/E_AnimState Enum" :default "NewEnumerator0"))
  (message `/Game/Blueprints/Anim/BPI_PawnAnimation.SetAnimation` (`SkeletalMeshComponent.GetAnimInstance` (`self.SkeletalMesh`)) Animation))

(fn `UserConstructionScript`)