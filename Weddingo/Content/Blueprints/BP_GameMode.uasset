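; Game mode that assigns each joining player a specific spawn point.
; It overrides ChoosePlayerStart, gets the controller's index from BP_GameState, and scans all BP_PlayerStart actors for the one with that PlayerIndex and the first Scene enum value.
; The event graph and construction script are empty.
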(event `self.ReceiveBeginPlay`)

(fn `ChoosePlayerStart`
  (params (Player :type "Controller Object Reference"))
  (returns (ReturnValue :type "Actor Object Reference"))
  (bind _asplayer_controller (cast `PlayerController` Player))
  (bind _asbp_game_state (cast `/Game/Blueprints/BP_GameState` (`GameplayStatics.GetGameState`)))
  (bind _playerindex (`/Game/Blueprints/BP_GameState.GetPlayerIndex` _asbp_game_state _asplayer_controller))
  (bind _outactors (`GameplayStatics.GetAllActorsOfClass` "/Game/Blueprints/BP_PlayerStart.BP_PlayerStart_C"))
  (for _array_element _outactors
    (if (and (== (`/Game/Blueprints/BP_PlayerStart.playerIndex` _array_element) _playerindex) (`|EnumEquality` (`/Game/Blueprints/BP_PlayerStart.Scene` _array_element) "NewEnumerator0"))
      (return _array_element))))

(fn `UserConstructionScript`)