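; Player controller that sets up Enhanced Input and game-only input mode with a visible mouse cursor.
; BeginPlay waits briefly, then adds the default mapping context and applies those input settings.
; The Attack_Me input action asks BP_GameState for this controller's player index and prints it to screen, apparently as a multiplayer identity check.
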(event `self.ReceiveBeginPlay`
  (`KismetSystemLibrary.Delay` 0.2)
  (`EnhancedInputSubsystemInterface.AddMappingContext` (pcsubsystem `EnhancedInputLocalPlayerSubsystem` self) "/Game/Inputs/IMP_Default.IMP_Default" 0 (struct))
  (`WidgetBlueprintLibrary.SetInputMode_GameOnly` self)
  (set `self.bShowMouseCursor` true))

(event `EnhancedInput|/Game/Inputs/IA_Attack_Me`
  (params (ActionValue :type Boolean) (ElapsedSeconds :type "Float (double-precision)") (TriggeredSeconds :type "Float (double-precision)") (InputAction :type "InputAction Object Reference" :default "/Game/Inputs/IA_Attack_Me.IA_Attack_Me"))
  (:`Triggered`
    (bind _asbp_game_state (cast `/Game/Blueprints/BP_GameState` (`GameplayStatics.GetGameState`)))
    (bind _playerindex (`/Game/Blueprints/BP_GameState.GetPlayerIndex` _asbp_game_state self))
    (`KismetSystemLibrary.PrintString` (`KismetStringLibrary.Concat_StrStr` "I am player " (`KismetStringLibrary.Conv_IntToString` _playerindex)))))

(fn `UserConstructionScript`)