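; BP_Transition is an actor that plays a screen transition effect through a post-process material.
; Its Start event creates a dynamic instance of Transition_Inst, enables the PostProcess component and adds the instance as a full-weight blendable.
; A timeline then plays from the start, driving the material's Ratio scalar parameter on each update.
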(event `Start`
  (bind _postprocess (`self.PostProcess`))
  (bind _returnvalue (`KismetMaterialLibrary.CreateDynamicMaterialInstance` "/Game/Animations/Transition_Inst.Transition_Inst"))
  (set `self.MatInst` _returnvalue)
  (set `PostProcessComponent.bEnabled` true _postprocess)
  (`KismetArrayLibrary.Array_Add` (`.Array` (break `WeightedBlendables` (`.WeightedBlendables` (break `PostProcessSettings` (`PostProcessComponent.Settings` _postprocess))))) (make `WeightedBlendable` 1.0 (`self.MatInst`)))
  (bind (_direction _ratio) (`Timeline|Timeline` :!via `PlayFromStart`)
    (:`Update`
      (`MaterialInstanceDynamic.SetScalarParameterValue` (`self.MatInst`) "Ratio" _ratio))))

(fn `UserConstructionScript`)