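; Game state that runs a local two-player question game, where a round is won when the players' "selected me" answers differ, meaning they agree on one person.
; It loads questions from DT_Questions, shows each on the HUD, starts both controllers' rounds, then records and displays the result.
; When the next question's scene differs, it fades, switches camera and level, and teleports pawns to that scene's player starts before resuming on OnTransitionEnd.
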(event `self.ReceiveBeginPlay`
  (`GameplayStatics.CreatePlayer` -1)
  (`self.RetrieveAllQuestions`)
  (bind _returnvalue (`|CreateWidget` "/Game/HUD/BP_HUD.BP_HUD_C"))
  (bind _output_get (set `self.HUD` _returnvalue))
  (`UserWidget.AddToViewport` _output_get 0)
  (`self.StartGame`))

(event `StartGame`
  (`self.AskQuestion`))

(event `AskQuestion`
  (bind _output (`self.GetCurrentQuestion`))
  (`self.SendQuestionToHUD` _output)
  (for _array_element (`self.PlayerArray`)
    (bind _asbp_player_controller (cast `/Game/Blueprints/BP_PlayerController` (`PlayerState.GetPlayerController` _array_element)))
    (`/Game/Blueprints/BP_PlayerController.StartRound` _asbp_player_controller)))

(event `ReceiveAnswer`
  (params (SelectedMe :type Boolean))
  (`KismetArrayLibrary.Array_Add` (`self.Answers`) SelectedMe)
  (if (== (`KismetArrayLibrary.Array_Length` (`self.Answers`)) 2)
    (`self.Result`)))

(event `Cheat`
  (bind _answers (`self.Answers`))
  (`KismetArrayLibrary.Array_Add` _answers)
  (`KismetArrayLibrary.Array_Add` _answers true)
  (`self.Result`))

(event `Result`
  (bind _hud (`self.HUD`))
  (bind _success (`self.CompareAnswers`))
  (`KismetArrayLibrary.Array_Add` (`self.Recap`) _success)
  (if _success
    (`/Game/HUD/BP_HUD.Victory` _hud)
    (else
      (`/Game/HUD/BP_HUD.Defeat` _hud)))
  (`KismetSystemLibrary.Delay` 3.0)
  (`/Game/HUD/BP_HUD.ResetQuestion` (`self.HUD`))
  (`self.NextQuestion`))

(event `NextQuestion`
  (`KismetArrayLibrary.Array_Clear` (`self.Answers`))
  (`/Engine/EditorBlueprintResources/StandardMacros.IncrementInt` (`self.CurrentQuestionIndex`)
    (:`  `
      (bind _returnvalue (`self.HasQuestion`))
      (if _returnvalue
        (bind _returnvalue_2 (`self.NeedTransition`))
        (if _returnvalue_2
          (`self.Transition`)
          (else
            (`self.AskQuestion`)))
        (else
          (`self.TheEnd`))))))

(event `Transition`
  (`self.Fade`)
  (`KismetSystemLibrary.Delay` 1.0)
  (`self.SetCurrentScene`)
  (`self.TransitionCamera`)
  (`self.RespawnPawns`))

(event `OnTransitionEnd`
  (`self.AskQuestion`))

(event `TheEnd`)

(fn `CompareAnswers`
  (returns (Success :type Boolean))
  (locals (firstAnswer :type Boolean))
  (for (_array_element _array_index) (`self.Answers`)
    (if (== _array_index 0)
      (set `local.firstAnswer` _array_element)
      (else
        (return (!= _array_element (`local.firstAnswer`)))))))

(fn `Fade`
  (bind _outactors (`GameplayStatics.GetAllActorsOfClass` "/Game/Blueprints/BP_Transition.BP_Transition_C"))
  (for _array_element _outactors
    (`/Game/Blueprints/BP_Transition.Start` _array_element)))

(fn `GetCurrentQuestion`
  (returns (Output :type "/Game/Data/S_Question Structure (by ref)"))
  (return (`|GetArrayItem` (`self.Questions`) (`self.CurrentQuestionIndex`))))

(fn `GetPlayerIndex`
  (params (PlayerController :type "PlayerController Object Reference"))
  (returns (PlayerIndex :type Integer))
  (for (_array_element _array_index) (`self.PlayerArray`)
    (if (== (`PlayerState.GetPlayerController` _array_element) PlayerController)
      (return _array_index)))
  (return -1))

(fn `HasQuestion`
  (returns (ReturnValue :type Boolean))
  (return (< (`self.CurrentQuestionIndex`) (`KismetArrayLibrary.Array_Length` (`self.Questions`)))))

(fn `NeedTransition`
  (returns (ReturnValue :type Boolean))
  (bind (_output_text _output_scene) (break `/Game/Data/S_Question` (`|GetArrayItem` (`self.Questions`) (`self.CurrentQuestionIndex`))))
  (return (`|EnumInequality` (`self.CurrentScene`) _output_scene)))

(fn `RespawnPawns`
  (bind _outactors (`GameplayStatics.GetAllActorsOfClass` "/Game/Blueprints/BP_PlayerStart.BP_PlayerStart_C"))
  (for _array_element _outactors
    (if (`|EnumEquality` (`/Game/Blueprints/BP_PlayerStart.Scene` _array_element) (`self.CurrentScene`))
      (for _array_element_2 (`self.PlayerArray`)
        (bind _returnvalue (`PlayerState.GetPlayerController` _array_element_2))
        (bind _asbp_player_controller (cast `/Game/Blueprints/BP_PlayerController` _returnvalue))
        (bind _playerindex (`self.GetPlayerIndex` _asbp_player_controller))
        (if (== _playerindex (`/Game/Blueprints/BP_PlayerStart.playerIndex` _array_element))
          (`self.K2_SetActorTransform` (`Controller.K2_GetPawn` _returnvalue) (`self.GetTransform` _array_element) false true))))))

(fn `RetrieveAllQuestions`
  (bind _outrownames (`DataTableFunctionLibrary.GetDataTableRowNames` "/Game/Data/DT_Questions.DT_Questions"))
  (for _array_element _outrownames
    (bind _returnvalue (`|GetDataTableRow` "/Game/Data/DT_Questions.DT_Questions" _array_element)
      (:`then`
        (`KismetArrayLibrary.Array_Add` (`self.Questions`) _returnvalue)))))

(fn `SendQuestionToHUD`
  (params (S_Question :type "/Game/Data/S_Question Structure (by ref)"))
  (`/Game/HUD/BP_HUD.SetQuestion` (`self.HUD`) (`.Text_2_10DA53D441B2B94DF7927BB7F623BA0A` (break `/Game/Data/S_Question` S_Question))))

(fn `SetCurrentScene`
  (set `self.CurrentScene` (`.Scene_6_D8B7EA664C76E12B664054AE30EB19A0` (break `/Game/Data/S_Question` (`|GetArrayItem` (`self.Questions`) (`self.CurrentQuestionIndex`)))))
  (return))

(fn `TransitionCamera`
  (bind _outactors (`GameplayStatics.GetAllActorsOfClass` "/Game/Blueprints/BP_SceneCamera.BP_SceneCamera_C"))
  (for _array_element _outactors
    (if (`|EnumEquality` (`/Game/Blueprints/BP_SceneCamera.Scene` _array_element) (`self.CurrentScene`))
      (bind _asbp_player_controller (cast `/Game/Blueprints/BP_PlayerController` (`GameplayStatics.GetPlayerController` 0)))
      (`/Game/Blueprints/BP_PlayerController.CameraTransition` _asbp_player_controller _array_element)))
  (`self.RequestLevelTransition` (`self.CurrentScene`)))

(fn `UserConstructionScript`)