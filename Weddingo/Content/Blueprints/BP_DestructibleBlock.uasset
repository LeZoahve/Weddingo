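; BP_DestructibleBlock triggers Chaos destruction within a spherical area shortly after play begins.
; The construction script offsets and sizes the sphere from height and radius variables.
; After a brief delay, the Field System applies external cluster strain through a radial falloff to break clusters.
; It then applies radial linear velocity, culled outside the sphere and scaled by DestructionAmplitude, to push pieces from the centre.
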(event `self.ReceiveBeginPlay`
  (bind _fieldsystem (`self.FieldSystem`))
  (bind _sphere (`self.Sphere`))
  (bind _returnvalue (`SceneComponent.K2_GetComponentLocation` _sphere))
  (bind _returnvalue_2 (`RadialFalloff.SetRadialFalloff` (`self.RadialFalloff`) 500000.0 1.0 1.0 0.0 (`SphereComponent.GetScaledSphereRadius` _sphere) _returnvalue "Field_FallOff_None"))
  (`KismetSystemLibrary.Delay` 0.5)
  (`FieldSystemComponent.ApplyPhysicsField` _fieldsystem true "Field_ExternalClusterStrain" null _returnvalue_2)
  (`FieldSystemComponent.ApplyPhysicsField` _fieldsystem true "Field_LinearVelocity" null (`CullingField.SetCullingField` (`self.CullingField`) _returnvalue_2 (`RadialVector.SetRadialVector` (`self.RadialVector`) (`KismetMathLibrary.Conv_IntToDouble` (`self.DestructionAmplitude`)) _returnvalue) "Field_Culling_Outside")))

(fn `UserConstructionScript`
  (`SceneComponent.K2_AddLocalOffset` (`self.Sphere`) (`KismetMathLibrary.MakeVector` 0.0 0.0 (`KismetMathLibrary.Conv_IntToDouble` (`self.SphereHeight`))) false false)
  (`SphereComponent.SetSphereRadius` (`self.Sphere`) (`KismetMathLibrary.Conv_IntToDouble` (`self.SphereRadius`)) true))